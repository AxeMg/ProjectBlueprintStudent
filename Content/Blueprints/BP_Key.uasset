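; BP_Key is a pickup key actor that the player collects through an Interaction event.
; Interaction sets the entry at IdKey in the player's Keys array to true, then destroys the key.
; When IdKey is 1, it also unlocks the referenced OpenDoor and triggers that door's Interaction.
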(event `/Game/BPI_Interaction.Interaction`
  (bind _opendoor (`self.OpenDoor`))
  (`KismetArrayLibrary.Array_Set` (`/Game/BP_Player.Keys` (cast `/Game/BP_Player` (`GameplayStatics.GetPlayerCharacter` 0) :!pure true)) (`self.IdKey`) true)
  (`self.K2_DestroyActor`)
  (if (== (`self.IdKey`) 1)
    (set `/Game/BP_Door.IsLocked` false _opendoor)
    (`/Game/BPI_Interaction.Interaction` _opendoor)))

(fn `UserConstructionScript`)