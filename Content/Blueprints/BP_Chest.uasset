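; Chest actor that opens only when every entry in the player's Keys array is true.
; The check runs on both BeginPlay and the Interaction event.
; On success, timelines slide and rotate two key meshes, the second started from the first's Update, while a third timeline swings the lid open in parallel.
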(event `self.ReceiveBeginPlay`
  (bind _sm_key (`self.SM_Key`))
  (bind _sm_key1 (`self.SM_Key1`))
  (bind _returnvalue (`SceneComponent.GetRelativeTransform` _sm_key1))
  (bind _returnvalue_2 (`SceneComponent.GetRelativeTransform` _sm_key))
  ;[1 1 1] Verif si on a les cle
  (set `self.CanOpen` true :!label _label)
  (for _array_element (`/Game/BP_Player.Keys` (cast `/Game/BP_Player` (`GameplayStatics.GetPlayerCharacter` 0) :!pure true))
    (if (not _array_element)
      (set `self.CanOpen` false)))
  (if (`self.CanOpen`)
    (`|ExecutionSequence`
      (:`then_0`
        ;[1 1 1] Anim de la cle
        (bind (_direction _movement _rotation) (`Timeline|Timeline`)
          (:`Update`
            (`SceneComponent.K2_SetRelativeLocationAndRotation` _sm_key (`KismetMathLibrary.MakeVector` (.x (.location _returnvalue_2)) (`KismetMathLibrary.Lerp` 107.0 85.0 _movement) (.z (.location _returnvalue_2))) (`KismetMathLibrary.MakeRotator` (.roll (.rotation _returnvalue_2)) (`KismetMathLibrary.Lerp` -90.0 0.0 _rotation) (.yaw (.rotation _returnvalue_2))) false false)
            ;[1 1 1] Anim de la cle
            (bind (_direction_2 _movement_2 _rotation_2) (`Timeline|Timeline_0`)
              (:`Update`
                (`SceneComponent.K2_SetRelativeLocationAndRotation` _sm_key1 (`KismetMathLibrary.MakeVector` (.x (.location _returnvalue)) (`KismetMathLibrary.Lerp` 107.0 85.0 _movement_2) (.z (.location _returnvalue))) (`KismetMathLibrary.MakeRotator` (.roll (.rotation _returnvalue)) (`KismetMathLibrary.Lerp` -90.0 0.0 _rotation_2) (.yaw (.rotation _returnvalue))) false false))))))
      (:`then_1`
        ;[1 1 1] Ouverture du coffre
        (bind (_direction_3 _chestrotation) (`Timeline|ChestOpen`)
          (:`Update`
            (`SceneComponent.K2_SetRelativeRotation` (`self.Chest_cover_StaticMeshComponent0`) (`KismetMathLibrary.MakeRotator` (`KismetMathLibrary.Lerp` 0.0 -60.0 _chestrotation)) false false)))))))

(event `/Game/BPI_Interaction.Interaction`
  (goto _label))

(fn `UserConstructionScript`)